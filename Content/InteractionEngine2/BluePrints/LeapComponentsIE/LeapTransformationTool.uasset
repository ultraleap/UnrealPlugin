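; Leap hand-interaction grab component that lets a hand slide its owning actor along one of the actor's local axes.
; TryGrab picks the axis most aligned with the hand's offset from the actor, fires the grabbed callback and plays left-hand haptics.
; A 0.01-second looping timer projects the hand-to-collision-surface gap, with slight padding, onto that axis and offsets the actor.
; TryRelease pauses the timer and resets the axis selection threshold.
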(event Custom|OnGrabbing
  (CallFunction|OnGrabbingTriggered))

(event Custom|OnGrabbingTriggered
  (bind _returnvalue (Components|GetOwner))
  (bind _returnvalue_2 (Components|GetOwner))
  (bind _returnvalue_3 (Components|GetOwner))
  (bind _returnvalue_4 (Components|GetOwner))
  (bind _hand (Variables|Default|GetHand))
  (bind _handattachsocket (Variables|Default|GetHandAttachSocket))
  (bind _returnvalue_5 (Transformation|GetSocketLocation _hand _handattachsocket))
  (bind _returnvalue_6 (Transformation|GetActorUpVector _returnvalue_3))
  (bind _returnvalue_7 (Transformation|GetActorRightVector _returnvalue_4))
  (bind _returnvalue_8 (Transformation|GetActorForwardVector _returnvalue))
  (if (Variables|Default|GetbIsHeld)
    (Utilities|IsValid _returnvalue_2
      (:Is%20Valid
        (bind _asprimitive_component (Utilities|Casting|CastToPrimitiveComponent (Variables|/Script/Engine.Actor|GetRootComponent _returnvalue_2)))
        (switch Utilities|FlowControl|Switch|SwitchonLeapTransformDirection (Variables|Default|GetDirection)
          (:NewEnumerator0
            (Variables|Default|SetDeltaLocation (* _returnvalue_6 (Math|Vector|DotProduct _returnvalue_6 (- _returnvalue_5 (+ (* (Math|Vector|Normalize (- (.OutPointOnBody (Collision|GetClosestPointonCollision _asprimitive_component _returnvalue_5 "None")) (Transformation|GetActorLocation (Components|GetOwner)))) 2.0) (.OutPointOnBody (Collision|GetClosestPointonCollision _asprimitive_component _returnvalue_5 "None"))))))))
          (:NewEnumerator1
            (Variables|Default|SetDeltaLocation (* _returnvalue_7 (Math|Vector|DotProduct (- _returnvalue_5 (+ (* (Math|Vector|Normalize (- (.OutPointOnBody (Collision|GetClosestPointonCollision _asprimitive_component _returnvalue_5 "None")) (Transformation|GetActorLocation (Components|GetOwner)))) 2.0) (.OutPointOnBody (Collision|GetClosestPointonCollision _asprimitive_component _returnvalue_5 "None")))) _returnvalue_7))))
          (:NewEnumerator2
            (Variables|Default|SetDeltaLocation (* _returnvalue_8 (Math|Vector|DotProduct (- _returnvalue_5 (+ (* (Math|Vector|Normalize (- (.OutPointOnBody (Collision|GetClosestPointonCollision _asprimitive_component _returnvalue_5 "None")) (Transformation|GetActorLocation (Components|GetOwner)))) 2.0) (.OutPointOnBody (Collision|GetClosestPointonCollision _asprimitive_component _returnvalue_5 "None")))) _returnvalue_8)))))
        (Transformation|AddActorWorldOffset (Components|GetOwner) (Variables|Default|GetDeltaLocation))))))

(event EventBeginPlay
  (bind _returnvalue (Utilities|Time|SetTimerbyEvent (delegate Custom|OnGrabbing) 0.01 true))
  (bind _output_get (Variables|Default|SetGrabTimer _returnvalue))
  (Utilities|Time|PauseTimerbyHandle _output_get))

(fn TryGrab
  (params (MotionController :type Motion%20Controller%20Component%20Object%20Reference) (Hand :type Skeletal%20Mesh%20Component%20Object%20Reference) (LeftHandAttachSocket :type Name :default "None") (LeftHandBaseSocket :type Name :default "None") (RightHandBaseSocket :type Name :default "None") (RightHandAttachSocket :type Name :default "None") (HandType :type EHandType%20Enum :default "LEAP_HAND_LEFT"))
  (bind _returnvalue (Components|GetOwner))
  (bind _returnvalue_2 (Components|GetOwner))
  (bind _returnvalue_3 (Components|GetOwner))
  (bind _handattachsocket (Variables|Default|GetHandAttachSocket))
  (bind _returnvalue_4 (Transformation|GetSocketLocation (Variables|Default|GetHand) _handattachsocket))
  (bind _returnvalue_5 (Transformation|GetActorLocation _returnvalue))
  (bind _returnvalue_6 (Transformation|GetActorLocation _returnvalue_2))
  (bind _returnvalue_7 (Transformation|GetActorForwardVector _returnvalue_2))
  (bind _returnvalue_8 (Transformation|GetActorLocation _returnvalue_3))
  (bind _returnvalue_9 (Transformation|GetActorUpVector _returnvalue_3))
  (bind _returnvalue_10 (Transformation|GetActorRightVector _returnvalue))
  (bind _returnvalue_11 (- _returnvalue_4 _returnvalue_5))
  (bind _returnvalue_12 (- _returnvalue_4 _returnvalue_6))
  (bind _returnvalue_13 (- _returnvalue_4 _returnvalue_8))
  (bind _returnvalue_14 (Math|Vector|DotProduct _returnvalue_11 _returnvalue_10))
  (bind _returnvalue_15 (Math|Vector|DotProduct _returnvalue_12 _returnvalue_7))
  (bind _returnvalue_16 (Math|Vector|DotProduct _returnvalue_13 _returnvalue_9))
  (bind _returnvalue_17 (Math|Float|Absolute(Float) _returnvalue_15))
  (bind _returnvalue_18 (Math|Float|Absolute(Float) _returnvalue_16))
  (bind _returnvalue_19 (Math|Float|Absolute(Float) _returnvalue_14))
  (CallFunction|SetGrabVars Hand LeftHandBaseSocket LeftHandAttachSocket RightHandBaseSocket RightHandAttachSocket HandType)
  (Utilities|FlowControl|Sequence ; Try to grab, then continue
    (:then_0
      (switch Utilities|FlowControl|Switch|SwitchonGrabType (Variables|Default|GetGrabType)
        (:NewEnumerator7
          (Variables|Default|SetbIsHeld true)
          (Utilities|Time|UnpauseTimerbyHandle (Variables|Default|GetGrabTimer))
          (Variables|Default|SetInitialiHandLocation _returnvalue_4)
          (Utilities|FlowControl|Sequence
            (:then_0
              (if (> _returnvalue_17 (Variables|Default|GetMinDotProd))
                (Variables|Default|SetMinDotProd _returnvalue_17)
                (Variables|Default|SetDirection "NewEnumerator2")))
            (:then_1
              (if (> _returnvalue_18 (Variables|Default|GetMinDotProd))
                (Variables|Default|SetMinDotProd _returnvalue_18)
                (Variables|Default|SetDirection "NewEnumerator0")))
            (:then_2
              (if (> _returnvalue_19 (Variables|Default|GetMinDotProd))
                (Variables|Default|SetMinDotProd _returnvalue_19)
                (Variables|Default|SetDirection "NewEnumerator1")))))))
    (:then_1
      (if (Variables|Default|GetbIsHeld) ; Did the grab succeed?
        (Variables|Default|SetMotionControllerRef MotionController) ; Store a reference to the MotionController\nthat initiated the Grab
        (Default|CallOnGrabbed) ; Call the Event Dispatcher so that we can do custom logic\nin the Blueprint that implements this GrabComponent
        (Variables|Default|GetMotionControllerRef
          (:then
            (Class|PlayerController|PlayHapticEffect (Game|GetPlayerController 0) (Variables|Default|GetOnGrabHapticEffect) "Left" 1.0 false))
          (:else
            _))
        (return true) ; Return that we're held!
        (else
          (return false) ; Return that nothing is held
        )))))

(fn TryRelease
  (Variables|Default|SetbIsHeld false)
  (Variables|Default|SetInitialiHandLocation "0, 0, 0")
  (Utilities|Time|PauseTimerbyHandle (Variables|Default|GetGrabTimer))
  (Variables|Default|SetMinDotProd 0.0)
  (return true))